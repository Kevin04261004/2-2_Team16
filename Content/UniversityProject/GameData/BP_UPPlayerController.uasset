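; Player controller that handles the game over and game clear end states.
; On BeginPlay it caches the game mode and its HUD widget, then adds the game over widget to the viewport hidden; an uncalled Init function duplicates this setup.
; OnGameOver and OnGameClear trigger their matching widget, then stop the brain logic of the Pettu AI controller found by class lookup.
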(event EventBeginPlay
  (bind _wbp_gameover (Variables|Default|GetWBP%20GameOver))
  (bind _asbp_upgame_mode (Utilities|Casting|CastToBP_UPGameMode (Game|GetGameMode)))
  (bind _output_get (Variables|Default|SetAs%20BP%20UPGame%20Mode _asbp_upgame_mode))
  (bind _aswbp_hud (Utilities|Casting|CastToWBP_HUD (Variables|/Script/UniversityProject.UPGameMode|GetHudWidgetObject _output_get)))
  (Variables|Default|SetAs%20WBP%20HUD _aswbp_hud)
  (UserInterface|Viewport|AddtoViewport _wbp_gameover 0)
  (Widget|SetVisibility _wbp_gameover "Hidden"))

(event EventTick
  (params (DeltaSeconds :type Float%20%28single-precision%29)))

(event EventOnGameOver
  (Default|GameOver (Variables|Default|GetWBP%20GameOver))
  (bind _returnvalue (Actor|GetActorOfClass "/Game/UniversityProject/AI/BP_PettuAIController.BP_PettuAIController_C"))
  (AI|Logic|StopLogic (Variables|/Script/AIModule.AIController|GetBrainComponent _returnvalue) "GameOver"))

(event EventOnGameClear
  (Default|GameClear (Variables|Default|GetWBP%20GameClear))
  (bind _returnvalue (Actor|GetActorOfClass "/Game/UniversityProject/AI/BP_PettuAIController.BP_PettuAIController_C"))
  (AI|Logic|StopLogic (Variables|/Script/AIModule.AIController|GetBrainComponent _returnvalue) "GameClear"))

(fn ConstructionScript)

(fn Init
  (bind _wbp_gameover (Variables|Default|GetWBP%20GameOver))
  (bind _asbp_upgame_mode (Utilities|Casting|CastToBP_UPGameMode (Game|GetGameMode)))
  (bind _output_get (Variables|Default|SetAs%20BP%20UPGame%20Mode _asbp_upgame_mode))
  (bind _aswbp_hud (Utilities|Casting|CastToWBP_HUD (Variables|/Script/UniversityProject.UPGameMode|GetHudWidgetObject _output_get)))
  (Variables|Default|SetAs%20WBP%20HUD _aswbp_hud)
  (UserInterface|Viewport|AddtoViewport _wbp_gameover 0)
  (Widget|SetVisibility _wbp_gameover "Hidden"))